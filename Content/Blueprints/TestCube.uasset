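; TestCube is a practice actor Blueprint that exercises variables, operators, conditions, custom events and components.
; AddScore and TakeDamage events update Score and Health, then print the new value.
; Disconnected, labelled snippets demonstrate score math, a win check, event calls, cube color and light radius changes, and an actor offset.
; None of these snippets run, and both BeginPlay and the construction script are empty.
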(event `self.ReceiveBeginPlay`)

(event `AddScore`
  (params (Amount :type Integer))
  (bind _output_get (set `self.Score` (+ (`self.Score`) Amount)))
  (`KismetSystemLibrary.PrintString` (`KismetStringLibrary.Conv_IntToString` _output_get)))

(event `TakeDamage`
  (params (DamageAmount :type Integer))
  (bind _output_get (set `self.Health` (- (`self.Health`) DamageAmount)))
  (`KismetSystemLibrary.PrintString` (`KismetStringLibrary.Conv_IntToString` _output_get)))

(fn `UserConstructionScript`)